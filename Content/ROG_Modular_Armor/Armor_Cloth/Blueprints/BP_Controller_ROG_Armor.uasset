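; Player controller for the ROG modular armor pack that gives the player a toggleable armor selector menu.
; On BeginPlay it creates the BPW_Armor_Selector widget, adds it to the viewport and hides its canvas panel.
; Tab alternates through a FlipFlop between showing the panel with Game and UI input plus mouse cursor, and hiding it with game-only input and no cursor.
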(event `self.ReceiveBeginPlay`
  (bind _returnvalue (`|CreateWidget` "/Game/ROG_Modular_Armor/Armor_Cloth/Blueprints/BPW_Armor_Selector.BPW_Armor_Selector_C" self))
  (set `self.ArmorSelector` _returnvalue)
  (`UserWidget.AddToViewport` (`self.ArmorSelector`) 0)
  (`Widget.SetVisibility` (`/Game/ROG_Modular_Armor/Armor_Cloth/Blueprints/BPW_Armor_Selector.CanvasPanel_Selector` (`self.ArmorSelector`)) "Hidden"))

(event `Key|Tab`
  (params (Key :type "Key Structure"))
  (:`Pressed`
    (`/Engine/EditorBlueprintResources/StandardMacros.FlipFlop`
      (:`A`
        (`Widget.SetVisibility` (`/Game/ROG_Modular_Armor/Armor_Cloth/Blueprints/BPW_Armor_Selector.CanvasPanel_Selector` (`self.ArmorSelector`)) "Visible")
        (`WidgetBlueprintLibrary.SetInputMode_GameAndUIEx` self (`/Game/ROG_Modular_Armor/Armor_Cloth/Blueprints/BPW_Armor_Selector.CanvasPanel_Selector` (`self.ArmorSelector`)))
        (set `self.bShowMouseCursor` true))
      (:`B`
        (`Widget.SetVisibility` (`/Game/ROG_Modular_Armor/Armor_Cloth/Blueprints/BPW_Armor_Selector.CanvasPanel_Selector` (`self.ArmorSelector`)) "Hidden")
        (`WidgetBlueprintLibrary.SetInputMode_GameOnly` self)
        (set `self.bShowMouseCursor` false)))))

(fn `UserConstructionScript`)